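; Cannonball projectile Blueprint that launches itself and passes its motion to a fluid simulation actor.
; On BeginPlay, after a zero-length delay, it sets a mostly upward velocity on its ProjectileMovementComponent.
; It then writes that velocity once to the first BP_FluidSimulation_01 found as force velocity, sets its radial force, and fills transform P from the velocity vector rather than the ball's position.
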(event EventBeginPlay
  (Utilities|FlowControl|Delay 0.0)
  (bind _output_get (Variables|/Script/Engine.MovementComponent|SetVelocity (Actor|GetComponentbyClass "/Script/Engine.ProjectileMovementComponent") (Math|Vector|MakeVector 0.0 -5.0 7e+02)))
  (bind _output_get_2 (Variables|Default|SetBallVelocity _output_get))
  (bind _outactors (Actor|GetAllActorsOfClass "/ShaderBits-GDC-Pack/FluidSimulation/Blueprints/BP_FluidSimulation_01.BP_FluidSimulation_01_C"))
  (Variables|/ShaderBits-GDC-Pack/FluidSimulation/Blueprints/BP_FluidSimulation_01.BP_FluidSimulation_01_C|SetForce%20Velocity (Utilities|Array|Get(acopy) _outactors) _output_get_2)
  (Variables|/ShaderBits-GDC-Pack/FluidSimulation/Blueprints/BP_FluidSimulation_01.BP_FluidSimulation_01_C|SetRadial%20Force (Utilities|Array|Get(acopy) _outactors) 1.0)
  (Variables|/ShaderBits-GDC-Pack/FluidSimulation/Blueprints/BP_FluidSimulation_01.BP_FluidSimulation_01_C|SetP (Utilities|Array|Get(acopy) _outactors) (Math|Conversions|ToTransform(Vector) _output_get_2)))

(event Input|MouseEvents|RightMouseButton
  (params (Key :type Key%20Structure)))

(fn ConstructionScript)